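; Star Destroyer actor that flies under AI control to a Destination offset from its current location.
; On BeginPlay or MoveToDestination it waits briefly, turns to face the offset point, then uses AIMoveTo with pathfinding off.
; When the move finishes it levels out, keeping only its yaw.
; The NavigationVolume3D path-finding, waypoint-following and debug-sphere logic is present but disconnected, so it never runs.
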(event `self.ReceiveBeginPlay`
  (bind (_returnvalue_roll _returnvalue_pitch _returnvalue_yaw) (`KismetMathLibrary.BreakRotator` (`self.K2_GetActorRotation`)))
  ;[1 1 1] Fly along the path
  (`KismetSystemLibrary.Delay` 2.0 :!label _label)
  (`self.RotateToNextDestination`)
  (`AITask_MoveTo.AIMoveTo` (cast `AIController` (`self.GetController`) :!pure true) (+ (`self.K2_GetActorLocation`) (`self.Destination`)) null 20.0 "Disable" "Disable" false false false "Disable"
    (:`OnMoveFinished`
      (`self.K2_SetActorRotation` (`KismetMathLibrary.MakeRotator` 0.0 0.0 _returnvalue_yaw)))))

(event `MoveToDestination`
  ;[1 1 1] Fly along the path
  (`KismetSystemLibrary.PrintString` "Hello")
  (goto _label))

(fn `GetTargetLocation`
  (returns (Output :type "Vector Structure"))
  (return (`|GetArrayItem` (`self.Path`) (`self.PathIndex`))))

(fn `OnLocationReached`
  (`/Engine/EditorBlueprintResources/StandardMacros.IncrementInt` (`self.PathIndex`)))

(fn `RotateToNextDestination`
  (bind _returnvalue (`self.K2_GetActorLocation`))
  (bind (_returnvalue_roll _returnvalue_pitch _returnvalue_yaw) (`KismetMathLibrary.BreakRotator` (`KismetMathLibrary.FindLookAtRotation` _returnvalue (+ _returnvalue (`self.Destination`)))))
  (`self.K2_SetActorRotation` (`KismetMathLibrary.MakeRotator` _returnvalue_roll _returnvalue_pitch _returnvalue_yaw)))

(fn `UserConstructionScript`)